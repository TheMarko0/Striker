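; BP_GameManager runs the Striker game loop, spawning BP_Cube AI pawns and tracking how many are killed.
; On BeginPlay it resets the kill count, creates the HUD widget and starts a looping timer that spawns cubes at random points on a flat box centred on SpawnArea.
; It passes itself to the HUD and each cube, and IncrementCubesKilled raises the count and refreshes the HUD score.
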(event `self.ReceiveBeginPlay`
  (`|ExecutionSequence`
    (:`then_0`
      (`self.Restart`)
      (bind _returnvalue (`|CreateWidget` "/Game/Striker/UI/WBP_HUD.WBP_HUD_C"))
      (`UserWidget.AddToViewport` _returnvalue 0)
      (set `/Game/Striker/UI/WBP_HUD.GameManager` self _returnvalue)
      (bind _output_get (set `self.HUDWidget` _returnvalue))
      (`/Game/Striker/UI/WBP_HUD.Update Score` _output_get))
    (:`then_1`
      (`KismetSystemLibrary.K2_SetTimer` null "Spawn Cube" 1.0 true))))

(event `self.ReceiveTick`
  (params (DeltaSeconds :type "Float (single-precision)")))

(fn ` Increment Cubes Killed`
  (`/Engine/EditorBlueprintResources/StandardMacros.IncrementInt` (`self.KilledCubes`)
    (:`  `
      (`/Game/Striker/UI/WBP_HUD.Update Score` (`self.HUDWidget`)))))

(fn `restart`
  (set `self.KilledCubes` 0))

(fn `Spawn Cube`
  (bind _returnvalue (`AIBlueprintHelperLibrary.SpawnAIFromClass` "/Game/Striker/Blueprints/BP_Cube.BP_Cube_C" null (`KismetMathLibrary.RandomPointInBoundingBox` (`KismetSystemLibrary.GetComponentBounds` (`self.SpawnArea`)) (1000.0 1000.0 0.0)) (struct) false null))
  (bind _ascube (cast `/Game/Striker/Blueprints/BP_Cube` _returnvalue))
  (set `/Game/Striker/Blueprints/BP_Cube.GameManager` self _ascube))

(fn `UserConstructionScript`)